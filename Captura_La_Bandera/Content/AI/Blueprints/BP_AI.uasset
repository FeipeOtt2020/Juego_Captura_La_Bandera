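; AI soldier for team deathmatch that roams random navmesh points and fights pawns of the opposing team.
; PawnSensing checks team via BPI_Team_Interaction, then chases with AIMoveTo and fires on arrival.
; A fire montage notify triggers muzzle effects and a sphere trace that applies damage.
; Death ragdolls the mesh and decrements the GameState team count, while Tick updates the health bar and turns both widgets toward the camera.
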(event `self.ReceiveBeginPlay`
  (`self.Search Around`)
  (`|ExecutionSequence`
    (:`then_0`
      (if (== (`self.Team`) 1)
        (bind _aswb_ai_team (cast `/Game/UI/HUD/WB_AI_Team` (`WidgetComponent.GetWidget` (`self.Team_Widget`))))
        (bind _teamtext (`/Game/UI/HUD/WB_AI_Team.TeamText` _aswb_ai_team))
        (`TextBlock.SetText` _teamtext "TEAM B")
        (`TextBlock.SetColorAndOpacity` _teamtext (make `SlateColor` (struct :`R` 0.325496 :`G` 0.838542 :`A` 1.0)))))
    (:`then_1`
      (`KismetSystemLibrary.Delay` 1.5 :!label _label)
      (if (`self.Has_Seen_Target`)
        (`self.Search Around`)
        (set `self.Has_Seen_Target` false)
        (goto _label)))))

(event `Search Around`
  ;[0.05098 0.05098 0.05098] Search around
  (if (not (`self.Has_Seen_Target`))
    (`|AIMoveTo` self (`NavigationSystemV1.K2_GetRandomReachablePointInRadius` (`self.K2_GetActorLocation`) 2000.0 null null) null 300.0
      (:`OnSuccess`
        (`KismetSystemLibrary.Delay` 1.0)
        (`self.Search Around`)))))

(event `self.ReceiveAnyDamage`
  (params (Damage :type "Float (single-precision)") (DamageType :type "DamageType Object Reference") (InstigatedBy :type "Controller Object Reference") (DamageCauser :type "Actor Object Reference"))
  ;[0.05098 0.05098 0.05098] AI_Health
  (set `self.AI_Health` (- (`self.AI_Health`) Damage))
  (if (<= (`self.AI_Health`) 0.0)
    (`/Engine/EditorBlueprintResources/StandardMacros.DoOnce` false
      (:`Completed`
        (`PrimitiveComponent.SetSimulatePhysics` (`self.Mesh`) true)
        (`CharacterMovementComponent.SetMovementMode` (`self.CharacterMovement`) "MOVE_None" 0)
        (set `self.Is_Dead` true)
        (`SceneComponent.SetVisibility` (`self.Health_Bar_Widget`) false false)
        (`SceneComponent.SetVisibility` (`self.Team_Widget`) false false)
        (bind _asgs_team_deathmatch (cast `/Game/AI/Blueprints/GS_Team_Deathmatch` (`GameplayStatics.GetGameState`)))
        (`/Game/AI/Blueprints/GS_Team_Deathmatch.Decrease_Team_Number` _asgs_team_deathmatch (== (`self.Team`) 0))))))

(event `self.PawnSensing.OnSeePawn`
  (params (Pawn :type "Pawn Object Reference"))
  (if (`KismetSystemLibrary.DoesImplementInterface` Pawn "/Game/AI/Blueprints/BPI_Team_Interaction.BPI_Team_Interaction_C")
    (bind _team (message `/Game/AI/Blueprints/BPI_Team_Interaction.Get_Team` Pawn))
    (if (!= _team (`KismetMathLibrary.Conv_ByteToInt` (`self.Team`)))
      (bind _asbp_ai (cast `/Game/AI/Blueprints/BP_AI` Pawn)
        (:`then`
          (if (`/Game/AI/Blueprints/BP_AI.Is_Dead` _asbp_ai)
            (`self.Search Around`)
            (else
              (`self.Chase_Target` Pawn :!label _label_2)
              (set `self.Has_Seen_Target` true))))
        (:`CastFailed`
          (goto _label_2))))))

(event `Chase_Target`
  (params (TargetActor :type "Actor Object Reference"))
  (`|AIMoveTo` self (0.0 0.0 0.0) TargetActor 450.0
    (:`OnSuccess`
      (`self.AI_Fire` TargetActor))))

(event `AI_Fire`
  (params (`Target Actor` :type "Actor Object Reference"))
  (bind _returnvalue_location (`KismetMathLibrary.BreakTransform` (`SceneComponent.GetSocketTransform` (`self.AI_Rifle`) "b_gun_muzzleflash" "RTS_World")))
  (bind _returnvalue (`SceneComponent.K2_GetComponentRotation` (`self.Mesh`)))
  (if (not (`self.Is_Dead`))
    (`Controller.SetControlRotation` (`self.GetController`) (`KismetMathLibrary.FindLookAtRotation` (`self.K2_GetActorLocation`) (`self.K2_GetActorLocation` `Target Actor`)))
    (`|PlayMontage` (`self.Mesh`) "/Game/Shooter_Animations/Fire_Rifle_Ironsights_Montage.Fire_Rifle_Ironsights_Montage"
      (:`OnNotifyBegin`
        (`GameplayStatics.SpawnEmitterAttached` "/Game/InfinityBladeEffects/Effects/FX_Monsters/FX_Monster_Gruntling/Master/P_BackPack_MuzzleFlash.P_BackPack_MuzzleFlash" (`self.AI_Rifle`) "b_gun_muzzleflash" _returnvalue_location _returnvalue (0.2 0.2 0.2) "KeepWorldPosition" true "AutoRelease")
        (bind (_outhit _returnvalue_2) (`KismetSystemLibrary.SphereTraceSingle` _returnvalue_location (+ _returnvalue_location (* (`KismetMathLibrary.GetRightVector` _returnvalue) 3000.0)) 12.0 "TraceTypeQuery1"))
        (if _returnvalue_2
          (bind (_bblockinghit _binitialoverlap _time _distance _location _impactpoint _normal _impactnormal _physmat _hitactor) (`GameplayStatics.BreakHitResult` _outhit))
          (`GameplayStatics.ApplyDamage` _hitactor 5.0)
          (`GameplayStatics.SpawnEmitterAtLocation` "/Game/InfinityBladeEffects/Effects/FX_Monsters/FX_Monster_Troll/death/P_TrollDeathImpact.P_TrollDeathImpact" _impactpoint (`KismetMathLibrary.MakeRotFromX` _normal) (0.65 0.65 0.65) true "AutoRelease"))))))

(event `self.ReceiveTick`
  (params (DeltaSeconds :type "Float (single-precision)"))
  (bind _aswb_ai_heatth_bar (cast `/Game/UI/HUD/WB_AI_Heatth_Bar` (`WidgetComponent.GetWidget` (`self.Health_Bar_Widget`))))
  (`ProgressBar.SetPercent` (`/Game/UI/HUD/WB_AI_Heatth_Bar.HealthBarAI` _aswb_ai_heatth_bar) (/ (`self.AI_Health`) 100.0))
  (`SceneComponent.K2_SetWorldRotation` (`self.Health_Bar_Widget`) (`KismetMathLibrary.FindLookAtRotation` (`self.K2_GetActorLocation`) (`self.K2_GetActorLocation` (`GameplayStatics.GetPlayerCameraManager` 0))) false false)
  (`SceneComponent.K2_SetWorldRotation` (`self.Team_Widget`) (`KismetMathLibrary.FindLookAtRotation` (`self.K2_GetActorLocation`) (`self.K2_GetActorLocation` (`GameplayStatics.GetPlayerCameraManager` 0))) false false))

(event `/Game/AI/Blueprints/BPI_Team_Interaction.Set_Team`
  (params (Team :type "/Game/AI/Blueprints/E_Teams Enum" :default "NewEnumerator0"))
  (set `self.Team` Team))

(fn `Get_Team`
  (returns (Team :type "/Game/AI/Blueprints/E_Teams Enum"))
  (return (`self.Team`)))

(fn `UserConstructionScript`)